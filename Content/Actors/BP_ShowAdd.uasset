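; BP_ShowAdd is an actor that keeps an AppLovin MAX interstitial ad preloaded; it does not show ads itself, despite its name.
; Delegate events request an ad on SDK initialization and again whenever one is hidden or fails to display.
; Failed loads retry after a capped exponential backoff delay driven by RetryAttempt, which resets when a load succeeds.
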(event OnSdkInitializedDynamicDelegate(AppLovinMAXDelegate)
  (params (SdkConfiguration :type Sdk%20Configuration%20Structure%20%28by%20ref%29))
  (Class|AppLovinMAX|LoadInterstitial (Variables|Default|GetAd%20Unit%20Identifier)))

(event OnInterstitialAdLoadedDynamicDelegate(AppLovinMAXDelegate)
  (params (AdInfo :type Ad%20Info%20Structure%20%28by%20ref%29))
  (Variables|Default|SetRetryAttempt 0.0) ; Reset retry attempts
)

(event OnInterstitialAdHiddenDynamicDelegate(AppLovinMAXDelegate)
  (params (AdInfo :type Ad%20Info%20Structure%20%28by%20ref%29))
  (Class|AppLovinMAX|LoadInterstitial (Variables|Default|GetAd%20Unit%20Identifier)))

(event OnInterstitialAdDisplayFailedDynamicDelegate(AppLovinMAXDelegate)
  (params (AdInfo :type Ad%20Info%20Structure%20%28by%20ref%29) (AdError :type Ad%20Error%20Structure%20%28by%20ref%29))
  (Class|AppLovinMAX|LoadInterstitial (Variables|Default|GetAd%20Unit%20Identifier)))

(event OnInterstitialAdLoadFailedDynamicDelegate(AppLovinMAXDelegate)
  (params (AdInfo :type Ad%20Info%20Structure%20%28by%20ref%29) (AdError :type Ad%20Error%20Structure%20%28by%20ref%29))
  (bind _result (Math|Float|IncrementFloat (Variables|Default|GetRetryAttempt))
    (:%20%20
      (Utilities|FlowControl|Delay (Math|Float|Power 2.0 (Math|Float|Min(Float) _result 6.0)))
      (Class|AppLovinMAX|LoadInterstitial (Variables|Default|GetAd%20Unit%20Identifier)))))

(fn ConstructionScript)